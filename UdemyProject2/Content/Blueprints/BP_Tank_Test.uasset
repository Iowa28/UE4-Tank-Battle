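; Test tank Blueprint that turns player input into driving, camera orbit and firing.
; BeginPlay hands the tracks to TankMovement and the barrel and turret to TankAiming, which receive the move, turn and fire inputs.
; Aim axes rotate the azimuth gimbal and spring arm, scaled by frame time.
; Projectile assignment and track physical-material setup are disconnected, and the mesh-setting function has no caller here.
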(event `self.ReceiveBeginPlay`
  (`TankMovementComponent.Initialise` (`self.TankMovement`) (`self.LeftTrack`) (`self.RightTrack`))
  (`TankAimingComponent.Initialise` (`self.TankAiming`) (`self.Barrel`) (`self.Turret`)))

(event `InputAxis|AimAzimuth`
  (params (AxisValue :type "Float (single-precision)"))
  ;[1 1 1] Camera Input Binding
  (`SceneComponent.K2_AddLocalRotation` (`self.Azimuth Gimbal`) (`KismetMathLibrary.MakeRotator` 0.0 0.0 (* AxisValue (`GameplayStatics.GetWorldDeltaSeconds`) 50.0)) false false))

(event `InputAxis|TurnRight`
  (params (AxisValue :type "Float (single-precision)"))
  ;[1 1 1] Movement Input Binding
  (`TankMovementComponent.IntendTurnRight` (`self.TankMovement`) AxisValue))

(event `InputAxis|Move`
  (params (AxisValue :type "Float (single-precision)"))
  ;[1 1 1] Movement Input Binding
  (`TankMovementComponent.IntendMoveForward` (`self.TankMovement`) AxisValue))

(event `InputAxis|AimElevation`
  (params (AxisValue :type "Float (single-precision)"))
  ;[1 1 1] Camera Input Binding
  (`SceneComponent.K2_AddLocalRotation` (`self.SpringArm`) (`KismetMathLibrary.MakeRotator` 0.0 (* AxisValue (`GameplayStatics.GetWorldDeltaSeconds`) 50.0)) false false))

(event `InputAction|Fire`
  (params (Key :type "Key Structure"))
  ;[1 1 1] Fire
  (:`Pressed`
    (`TankAimingComponent.Fire` (`self.TankAiming`))))

(fn `SetStaticMeshes`
  (`StaticMeshComponent.SetStaticMesh` (`self.Barrel`) "/Game/Tank/tank_fbx_Barrel.tank_fbx_Barrel")
  (`StaticMeshComponent.SetStaticMesh` (`self.Turret`) "/Game/Tank/tank_fbx_Turret.tank_fbx_Turret"))

(fn `SetupTracks`)

(fn `UserConstructionScript`)